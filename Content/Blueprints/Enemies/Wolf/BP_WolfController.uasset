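; AI controller for the wolf enemy that runs BT_Wolf on BeginPlay and feeds its perception results into the Blackboard.
; Perception updates write any BP_DungeonCharacter to TargetActor without checking whether it is currently sensed, marked as a sight test.
; Target perception updates go through HandleSightSense, which sets or clears TargetActor for player sight stimuli and records LastKnownLocation when the player is seen.
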(event `self.ReceiveBeginPlay`
  (`self.RunBehaviorTree` "/Game/Blueprints/Enemies/Wolf/BT_Wolf.BT_Wolf"))

(event `self.AIPerception.OnPerceptionUpdated`
  (params (UpdatedActors :type "Array of Actor Object Reference (by ref)"))
  ; Test AI perception of sight
  (for _array_element UpdatedActors
    (bind _asbp_dungeon_character (cast `/Game/Blueprints/Player/BP_DungeonCharacter` _array_element))
    (`BlackboardComponent.SetValueAsObject` (`self.Blackboard`) "TargetActor" _asbp_dungeon_character)))

(event `self.AIPerception.OnTargetPerceptionUpdated`
  (params (Actor :type "Actor Object Reference") (Stimulus :type "AIStimulus Structure"))
  ; Test AI perception of sight
  (`self.HandleSightSense` Actor Stimulus))

(fn `HandleSightSense`
  (params (Actor :type "Actor Object Reference") (Stimulus :type "AIStimulus Structure"))
  (bind (_stimulus_age _stimulus_expirationage _stimulus_strength _stimulus_stimuluslocation _stimulus_receiverlocation _stimulus_tag _stimulus_bsuccessfullysensed) (break `AIStimulus` (`local.Stimulus`)))
  ; GOD ONLY KNOWS
  (bind _returnvalue (`AIPerceptionSystem.GetSenseClassForStimulus` Stimulus))
  (if (== _returnvalue "/Script/AIModule.AISense_Sight")
    (if (== (`self.Actor`) (`GameplayStatics.GetPlayerCharacter` 0))
      (`BlackboardComponent.SetValueAsObject` (`self.Blackboard`) "TargetActor" (`KismetMathLibrary.SelectObject` (`GameplayStatics.GetPlayerCharacter` 0) null _stimulus_bsuccessfullysensed))
      (if _stimulus_bsuccessfullysensed
        (`BlackboardComponent.SetValueAsVector` (`self.Blackboard`) "LastKnownLocation" _stimulus_stimuluslocation))
      (else
        (return)))
    (else
      (return))))

(fn `UserConstructionScript`)