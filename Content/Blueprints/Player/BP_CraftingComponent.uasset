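; Player crafting component that toggles a crafting menu on and off with a temporary debug key.
; It creates the CraftingMenu_WBP widget on BeginPlay.
; On open, it passes its CraftingRecipes to the widget, generates categories, adds it to the viewport, and shows the cursor with game-and-UI input.
; On close, it removes the widget and restores game-only input.
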(event `self.ReceiveBeginPlay`
  (bind _returnvalue (`|CreateWidget` "/Game/Crafting/HUD/CraftingMenu_WBP.CraftingMenu_WBP_C"))
  (set `self.CraftingWidget` _returnvalue))

(event `Key|One`
  (params (Key :type "Key Structure"))
  (bind _returnvalue (`GameplayStatics.GetPlayerController` 0))
  (bind _craftingwidget (`self.CraftingWidget`))
  (bind _craftingwidget_2 (`self.CraftingWidget`))
  ; Temprorary. Open with 1.
  (:`Pressed`
    (if (`Widget.IsVisible` (`self.CraftingWidget`))
      (set `PlayerController.bShowMouseCursor` false _returnvalue)
      (`WidgetBlueprintLibrary.SetInputMode_GameOnly` _returnvalue)
      (`Widget.RemoveFromParent` _craftingwidget)
      (else
        (set `/Game/Crafting/HUD/CraftingMenu_WBP.CraftingRecipes` (`self.CraftingRecipes`) _craftingwidget_2)
        (`/Game/Crafting/HUD/CraftingMenu_WBP.GenerateCategories` _craftingwidget_2)
        (set `PlayerController.bShowMouseCursor` true _returnvalue)
        (`WidgetBlueprintLibrary.SetInputMode_GameAndUIEx` _returnvalue null "DoNotLock" false)
        (`UserWidget.AddToViewport` _craftingwidget 0)))))