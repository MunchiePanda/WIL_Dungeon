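; Player inventory component that holds nine item slots, creates the inventory widget and handles item pickup.
; Pressing E sphere-traces around a point below the player for a BP_Item, then puts it into the first slot that is empty or can stack it up to 64.
; A successful pickup refreshes the widget and destroys the item.
; FindEmptySlot finds slots without thumbnails but is not called here, and the widget visibility toggle is disconnected.
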(event `self.ReceiveBeginPlay`
  ;[0.07784 0.05967 0.15 0.5] Set the inventory widget in the component bp to be used in the player bp
  (bind _returnvalue (`|CreateWidget` "/Game/Blueprints/UserInterface/InventoryUI.InventoryUI_C"))
  (set `self.InventoryWidget` _returnvalue)
  (`KismetArrayLibrary.Array_Resize` (`self.items`) 9)
  (`/Game/Blueprints/UserInterface/InventoryUI.LoadInventory` (`self.InventoryWidget`) self))

(event `Key|I`
  (params (Key :type "Key Structure"))
  ;[0.08877 0.03769 0.15 0.5] Press I to open Inventory
)

(event `Key|E`
  (params (Key :type "Key Structure"))
  (bind _returnvalue (- (`Actor.K2_GetActorLocation` (`GameplayStatics.GetPlayerCharacter` 0)) (0.0 0.0 1000.0)))
  ;[0.15 0 0.05028 0.5] Sphere trace hits the ststic mesh of the item then adds the item to the ui, then destroy it
  (:`Pressed`
    (bind _outhit (`KismetSystemLibrary.SphereTraceSingle` :`Start` _returnvalue :`End` _returnvalue :`Radius` 1000.0 :`TraceChannel` "TraceTypeQuery1" :`DrawDebugType` "ForDuration"))
    (bind _asbp_item (cast `/Game/Blueprints/Inventory/BP_Item` (`.HitActor` (`GameplayStatics.BreakHitResult` _outhit))))
    (for (_array_element _array_index) (`self.items`)
      (`/Engine/EditorBlueprintResources/StandardMacros.IsValid` _asbp_item
        (:`Is Valid`
          (bind (_name _stackable _quantity) (break `/Game/Blueprints/Inventory/S_ItemStructure` _array_element))
          (bind _item (`/Game/Blueprints/Inventory/BP_Item.Item` _asbp_item))
          (bind (_name_2 _stackable_2 _quantity_2) (break `/Game/Blueprints/Inventory/S_ItemStructure` _item))
          (bind _returnvalue_2 (+ _quantity _quantity_2))
          (if (and (`KismetTextLibrary.EqualEqual_TextText` _name _name_2) _stackable_2 (<= _returnvalue_2 64))
            (bind (_item_name _item_stackable _item_quantity _item_thumbnail _item_mesh) (break `/Game/Blueprints/Inventory/S_ItemStructure` (`/Game/Blueprints/Inventory/BP_Item.Item` _asbp_item)))
            (`KismetArrayLibrary.Array_Set` (`self.items`) _array_index (make `/Game/Blueprints/Inventory/S_ItemStructure` _item_name _item_stackable _returnvalue_2 _item_thumbnail _item_mesh))
            (`/Game/Blueprints/UserInterface/InventoryUI.LoadInventory` (`self.InventoryWidget`) self :!label _label)
            (`Actor.K2_DestroyActor` _asbp_item)
            (elif (== _quantity 0)
              (`KismetArrayLibrary.Array_Set` (`self.items`) _array_index _item)
              (goto _label))))))))

(fn `FindEmptySlot`
  (returns (FirstIndex :type Integer) (isAvailable :type Boolean))
  (for (_array_element _array_index) (`self.items`)
    (if (not (`KismetSystemLibrary.IsValid` (`.Thumbnail_11_5A8F03BE4A0BE448B1FE128F833E0B7C` (break `/Game/Blueprints/Inventory/S_ItemStructure` _array_element))))
      (return _array_index true)))
  (return 0 false))