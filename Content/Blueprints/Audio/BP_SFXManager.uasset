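; Audio manager actor that plays named SFX and ambience, surface-based footsteps, and the maze overexposure death countdown.
; Helper functions look up sounds in name-keyed maps and play, fade or adjust volume on a passed-in AudioComponent.
; Tick traces below the player and, while moving, plays the sound mapped to the surface type every frame.
; The countdown re-calls itself after a Delay that shortens as the count drops, speeding up the clicks.
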(event `BeginDeathCountDown`
  (bind _currentcount (`self.CurrentCount`))
  ; Countdown Noise when Player is about to die in the maze from over exposure
  (if (> _currentcount 0.0)
    (`GameplayStatics.PlaySound2D` "/Engine/VREditor/Sounds/VR_click3_Cue.VR_click3_Cue" 5.0 1.0 0.0 null null)
    (`KismetSystemLibrary.Delay` (`KismetMathLibrary.Lerp` 1.5 0.3 (`KismetMathLibrary.Conv_IntToDouble` (- 1 (/ _currentcount (`self.MazeStartCount`))))))
    (set `self.CurrentCount` (- _currentcount 1.0))
    (`self.BeginDeathCountDown`)))

(event `self.ReceiveBeginPlay`
  (bind _asbp_dungeon_character (cast `/Game/Blueprints/Player/BP_DungeonCharacter` (`GameplayStatics.GetPlayerCharacter` 0)))
  (set `self.PlayerRef` _asbp_dungeon_character)
  (`KismetSystemLibrary.LogString` "Player Ref Set")
  (`GameplayStatics.PlaySound2D` "/Engine/VREditor/Sounds/VR_click1_Cue.VR_click1_Cue" 1.0 1.0 0.0 null null)
  (set `self.CurrentCount` (`self.MazeStartCount`)))

(event `self.ReceiveTick`
  (params (DeltaSeconds :type "Float (single-precision)"))
  (bind _playerref (`self.PlayerRef`))
  (bind _returnvalue (`self.K2_GetActorLocation` _playerref))
  ; Plays Audio Based on the Surface that the Player is Stepping On.
  (bind _outhit (`KismetSystemLibrary.LineTraceSingle` _returnvalue (+ _returnvalue (* (`self.GetActorUpVector` _playerref) -200.0)) "TraceTypeQuery1"))
  (if (> (`KismetMathLibrary.VSizeSquared` (`self.GetVelocity` _playerref)) 0.1)
    (`GameplayStatics.PlaySoundAtLocation` (`BlueprintMapLibrary.Map_Find` (`self.PhysicalMaterialMap`) (`GameplayStatics.GetSurfaceType` _outhit)) (`self.K2_GetActorLocation` (`self.PlayerRef`)) (struct) 1.0 1.0 0.0 null null null null)))

(fn `AdjustVolume`
  (params (AudioComponent :type "AudioComponent Object Reference") (Volume :type "Float (double-precision)"))
  ; Adjust Volume of Selected Audio Component
  (`AudioComponent.AdjustVolume` AudioComponent 0.0 Volume "Logarithmic"))

(fn `PlayAmbience`
  (params (AudioComponent :type "AudioComponent Object Reference") (Name :type String))
  (bind (_value _returnvalue) (`BlueprintMapLibrary.Map_Find` (`self.AmbientMusicMap`) Name))
  ; Begin playing new Ambient Audio
  (if _returnvalue
    (`AudioComponent.SetSound` AudioComponent _value)
    (`AudioComponent.Play` AudioComponent 0.0)
    (else
      (`KismetSystemLibrary.LogString` "No Audio Found"))))

(fn `PlaySFX`
  (params (Name :type String) (AudioComponent :type "AudioComponent Object Reference"))
  (bind (_value _returnvalue) (`BlueprintMapLibrary.Map_Find` (`self.SFXMap`) Name))
  ; PlaysAudioFromSelectedAudioComponent
  (if _returnvalue
    (`AudioComponent.SetSound` AudioComponent _value)
    (`AudioComponent.Play` AudioComponent 0.0)
    (else
      (`KismetSystemLibrary.LogString` "No Audio Clip Found"))))

(fn `SwitchAmbience`
  (params (`Audio Component` :type "AudioComponent Object Reference") (FadeDuration :type "Float (double-precision)") (Name :type String))
  (bind (_value _returnvalue) (`BlueprintMapLibrary.Map_Find` (`self.AmbientMusicMap`) Name))
  ; Seamlessly Switch Ambient Music without Abruptness
  (`AudioComponent.FadeOut` `Audio Component` FadeDuration 0.0 "Linear")
  (if _returnvalue
    (`AudioComponent.SetSound` `Audio Component` _value)
    (`AudioComponent.FadeIn` `Audio Component` FadeDuration 1.0 0.0 "Linear")
    (else
      (`KismetSystemLibrary.LogString` "Audio Not Found"))))

(fn `UserConstructionScript`)